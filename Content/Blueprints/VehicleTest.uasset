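; VehicleTest is a test Blueprint that manages screen-sized render targets for per-pixel position and normal data.
; BeginPlay resizes PositionTexture and NormalTexture to the current viewport dimensions.
; CalcPixelPositionData draws PositionMaterial into PositionTexture, but neither event graph handler calls it.
; Tick is empty, and NormalTexture is only resized, never drawn to here.
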(event EventBeginPlay
  (bind _returnvalue (Viewport|GetViewportSize))
  (bind (_x _y) (Math|Vector2D|BreakVector2D _returnvalue))
  (bind _returnvalue_2 (Math|Float|Truncate _x))
  (bind _returnvalue_3 (Math|Float|Truncate _y))
  ;[1 1 1] Resize Texture To Fit The Viewport
  (Rendering|ResizeRenderTarget2D (Variables|Default|GetPositionTexture) _returnvalue_2 _returnvalue_3)
  (Rendering|ResizeRenderTarget2D (Variables|Default|GetNormalTexture) _returnvalue_2 _returnvalue_3))

(event EventTick
  (params (DeltaSeconds :type Float%20%28single-precision%29)))

(fn CalcPixelPositionData
  (Rendering|DrawMaterialtoRenderTarget (Variables|Default|GetPositionTexture) (Variables|Default|GetPositionMaterial)))