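; Map manager for what appears to be command-line-driven scene capture of buildings; BeginPlay currently only parses launch parameters into a struct and prints them.
; Unwired logic would pick a building by ID (position still zeroed), place a look-at CineCamera and render through Movie Pipeline Queue.
; Uncalled helpers save JSON and compute clamped 2D screen bounding boxes by projecting actor bounds corners, suggesting dataset annotation.
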(event EventBeginPlay
  (bind _params (CallFunction|GetCommandLineParams))
  (bind _output_get (Variables|Default|SetParams _params))
  (bind _outjsonstring (|StructtoJsonString _output_get))
  (Development|PrintString _outjsonstring true true "(R=0.167953,G=1.000000,B=0.000000,A=1.000000)" 5e+01))

(event EventTick
  (params (DeltaSeconds :type Float%20%28single-precision%29)))

(fn SetCameraHeightandPosition
  (params (BuildingPosition :type Vector))
  (bind (_x _y) (Math|Vector|BreakVector BuildingPosition))
  (Transformation|SetActorLocation (Variables|Default|GetCineCamera) (Math|Vector|MakeVector _x _y (.CamHeight (Utilities|Struct|BreakCmdParams (Variables|Default|GetParams)))) false false)
  (return))

(fn SelectBuidling
  (params (BuildingIndex :type Integer))
  (bind _buildings (Variables|Default|GetBuildings))
  (return "0, 0, 0" (Variables|/Game/Blueprints/Building.Building_C|GetCenter%20Position (Actor|GetComponentbyClass (Utilities|Array|Get(acopy) _buildings (Math|Integer|%(Integer) BuildingIndex (Utilities|Array|Length _buildings))) "/Game/Blueprints/Building.Building_C"))))

(fn SetCameraLookat
  (params (Camera%20Target :type Actor%20Soft%20Object%20Reference))
  (Variables|/Script/CinematicCamera.CineCameraActor|SetLookatTrackingSettings (Variables|Default|GetCineCamera) (Utilities|Struct|MakeCameraLookatTrackingSettings true false 1e+01 Camera%20Target))
  (return))

(fn SaveData
  (params (Data :type Object%20Object%20Reference) (FileName :type String) (FilePath :type String))
  (bind _outjsonstring (|StructtoJsonString Data))
  (bind _outjsonobject (Class|JsonBlueprintFunctionLibrary|FromString _outjsonstring))
  (Class|JsonBlueprintFunctionLibrary|ToFile _outjsonobject (Utilities|Struct|MakeFilePath (Utilities|String|Append FilePath "\"/\"" FileName)))
  (return))

(fn GetCommandLineParams
  (bind _returnvalue (Utilities|GetCommandLine))
  (Development|PrintString _returnvalue true true "(R=1.000000,G=0.000000,B=0.300493,A=1.000000)" 88.0)
  (Development|PrintString (Utilities|String|RightChop (.OutValue (Class|KismetSystemLibrary|ParseParamValue _returnvalue "OutputDir")) 1) true true "(R=1.000000,G=0.000000,B=0.300493,A=1.000000)" 88.0)
  (Development|PrintString (Utilities|String|RightChop (.OutValue (Class|KismetSystemLibrary|ParseParamValue _returnvalue "TimeOfDay")) 1) true true "(R=1.000000,G=0.000000,B=0.300493,A=1.000000)" 88.0)
  (return (Utilities|Struct|MakeCmdParams (Math|Conversions|ToInteger(Byte) (Utilities|String|RightChop (.OutValue (Class|KismetSystemLibrary|ParseParamValue _returnvalue "ResX")) 1)) (Math|Conversions|ToInteger(Byte) (Utilities|String|RightChop (.OutValue (Class|KismetSystemLibrary|ParseParamValue _returnvalue "ResY")) 1)) (Utilities|String|RightChop (.OutValue (Class|KismetSystemLibrary|ParseParamValue _returnvalue "OutputDir")) 1) (Math|Conversions|ToFloat(Integer) (Utilities|String|RightChop (.OutValue (Class|KismetSystemLibrary|ParseParamValue _returnvalue "CamHeight")) 1)) (Math|Conversions|ToInteger(Byte) (Utilities|String|RightChop (.OutValue (Class|KismetSystemLibrary|ParseParamValue _returnvalue "TimeOfDay")) 1)) (Math|Conversions|ToFloat(Integer) (Utilities|String|RightChop (.OutValue (Class|KismetSystemLibrary|ParseParamValue _returnvalue "FOV")) 1)) (Math|Conversions|ToInteger(Byte) (Utilities|String|RightChop (.OutValue (Class|KismetSystemLibrary|ParseParamValue _returnvalue "Weather")) 1)) (Math|Conversions|ToFloat(Integer) (Utilities|String|RightChop (.OutValue (Class|KismetSystemLibrary|ParseParamValue _returnvalue "CameraBlur")) 1)) (Math|Conversions|ToFloat(Integer) (Utilities|String|RightChop (.OutValue (Class|KismetSystemLibrary|ParseParamValue _returnvalue "ArrivalTime")) 1)) (Math|Conversions|ToFloat(Integer) (Utilities|String|RightChop (.OutValue (Class|KismetSystemLibrary|ParseParamValue _returnvalue "AtmosphericHaze")) 1)) (Math|Conversions|ToInteger(Byte) (Utilities|String|RightChop (.OutValue (Class|KismetSystemLibrary|ParseParamValue _returnvalue "CharacterCount")) 1)) (Math|Conversions|ToInteger(Byte) (Utilities|String|RightChop (.OutValue (Class|KismetSystemLibrary|ParseParamValue _returnvalue "ArmedCount")) 1)) (Math|Conversions|ToFloat(Integer) (Utilities|String|RightChop (.OutValue (Class|KismetSystemLibrary|ParseParamValue _returnvalue "RotationSpeed")) 1)) (Math|Conversions|ToInteger(Byte) (Utilities|String|RightChop (.OutValue (Class|KismetSystemLibrary|ParseParamValue _returnvalue "VehicleID")) 1)) (Math|Conversions|ToInteger(Byte) (Utilities|String|RightChop (.OutValue (Class|KismetSystemLibrary|ParseParamValue _returnvalue "BuildingID")) 1)) (Math|Conversions|ToInteger(Byte) (Utilities|String|RightChop (.OutValue (Class|KismetSystemLibrary|ParseParamValue _returnvalue "Mode")) 1)))))

(fn GetBBData
  (params (Actor :type Actor%20Object%20Reference))
  (bind (_origin _boxextent) (Collision|GetActorBounds Actor false false))
  (bind _returnvalue (Utilities|GetDisplayName Actor))
  (bind _xarray (Variables|Default|GetXArray))
  (bind _yarray (Variables|Default|GetYArray))
  (bind _cornerposition (Variables|Default|GetCornerPosition))
  (bind (_x _y _z) (Math|Vector|BreakVector _boxextent))
  (bind (_x_2 _y_2 _z_2) (Math|Vector|BreakVector _boxextent))
  (bind (_x_3 _y_3 _z_3) (Math|Vector|BreakVector _boxextent))
  (bind (_x_4 _y_4 _z_4) (Math|Vector|BreakVector _boxextent))
  (bind (_x_5 _y_5 _z_5) (Math|Vector|BreakVector _boxextent))
  (Utilities|Array|Clear (Variables|Default|GetCornerPosition))
  (Utilities|FlowControl|Sequence
    (:then_0
      (Utilities|Array|Add _cornerposition (+ _origin _boxextent))
      (Utilities|Array|Add _cornerposition (+ _origin (Math|Vector|MakeVector (* _x_5 -1.0) _y_5 _z_5)))
      (Utilities|Array|Add _cornerposition (+ _origin (Math|Vector|MakeVector _x_5 (* _y_5 -1.0) _z_5)))
      (Utilities|Array|Add _cornerposition (+ _origin (Math|Vector|MakeVector _x_5 _y_5 (* _z_5 -1.0))))
      (Utilities|Array|Add _cornerposition (+ _origin (Math|Vector|MakeVector (* _x_2 -1.0) _y_2 (* _z_2 -1.0))))
      (Utilities|Array|Add _cornerposition (+ _origin (Math|Vector|MakeVector (* _x_3 -1.0) (* _y_3 -1.0) _z_3)))
      (Utilities|Array|Add _cornerposition (+ _origin (Math|Vector|MakeVector _x_4 (* _y_4 -1.0) (* _z_4 -1.0))))
      (Utilities|Array|Add _cornerposition (+ _origin (Math|Vector|MakeVector (* _x -1.0) (* _y -1.0) (* _z -1.0)))))
    (:then_1
      (for _array_element _cornerposition
        (if (.ReturnValue (Class|GameplayStatics|ProjectWorldtoScreen (Game|GetPlayerController 0) _array_element false))
          (Utilities|Array|Add (Variables|Default|GetXArray) (.X (Math|Vector2D|BreakVector2D (.ScreenPosition (Class|GameplayStatics|ProjectWorldtoScreen (Game|GetPlayerController 0) _array_element false)))))
          (Utilities|Array|Add (Variables|Default|GetYArray) (.Y (Math|Vector2D|BreakVector2D (.ScreenPosition (Class|GameplayStatics|ProjectWorldtoScreen (Game|GetPlayerController 0) _array_element false)))))
          (Development|PrintString (Utilities|String|Append _returnvalue ":" (Utilities|String|ToString(Vector2d) (.ScreenPosition (Class|GameplayStatics|ProjectWorldtoScreen (Game|GetPlayerController 0) _array_element false)))) true true "(R=0.000000,G=0.660000,B=1.000000,A=1.000000)" 5.0)))
      (return (Utilities|Struct|MakeBBData _returnvalue (Math|Float|Clamp(Float) (.MinValue (Math|Float|MinOfFloatArray _xarray)) 0.0 6.4e+02) (Math|Float|Clamp(Float) (.MaxValue (Math|Float|MaxOfFloatArray _xarray)) 0.0 6.4e+02) (Math|Float|Clamp(Float) (.MinValue (Math|Float|MinOfFloatArray _yarray)) 0.0 512.0) (Math|Float|Clamp(Float) (.MaxValue (Math|Float|MaxOfFloatArray _yarray)) 0.0 512.0))))))

(fn GetWorldPosition)